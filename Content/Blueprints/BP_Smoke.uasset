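; BP_Smoke is Jett's smoke projectile, steered by the camera of the BP_Jett that instigates it.
; FireInDirection launches it, starts a short timer and turns on steering, so Tick re-aims its velocity along the camera's forward vector.
; A sphere hit or StopSmokeMovement ends steering, zeroes velocity and gravity, scales the sphere, then destroys the actor after a brief delay.
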(event `self.ReceiveBeginPlay`
  (bind _asbp_jett (cast `/Game/Blueprints/BP_Jett` (`self.GetInstigator`)))
  (set `self.JettChar` _asbp_jett))

(event `self.ReceiveTick`
  (params (DeltaSeconds :type "Float (single-precision)"))
  (if (`self.UpdateDirection`)
    (set `MovementComponent.Velocity` (* (`SceneComponent.GetForwardVector` (`/Game/Blueprints/BP_Jett.Camera` (`self.JettChar`))) (`ProjectileMovementComponent.InitialSpeed` (`self.ProjectileMovement`))) (`self.ProjectileMovement`))))

(event `Fire In Direction`
  (params (Direction :type "Vector Structure"))
  (bind _projectilemovement (`self.ProjectileMovement`))
  (set `MovementComponent.Velocity` (* Direction (`ProjectileMovementComponent.InitialSpeed` _projectilemovement)) _projectilemovement)
  (set `self.UpdateDirection` true)
  (`KismetSystemLibrary.K2_SetTimerDelegate` (`|CreateDelegate` :!event `Stop Smoke Movement`) 1.5))

(event `self.Sphere.OnComponentHit`
  (params (HitComponent :type "PrimitiveComponent Object Reference") (OtherActor :type "Actor Object Reference") (OtherComp :type "PrimitiveComponent Object Reference") (NormalImpulse :type "Vector Structure") (Hit :type "HitResult Structure (by ref)"))
  (bind _projectilemovement (`self.ProjectileMovement`))
  (set `self.UpdateDirection` false :!label _label)
  (set `MovementComponent.Velocity` (0.0 0.0 0.0) _projectilemovement)
  (set `ProjectileMovementComponent.ProjectileGravityScale` 0.0 _projectilemovement)
  (`SceneComponent.SetWorldScale3D` (`self.Sphere`) (2.0 2.0 2.0))
  (`KismetSystemLibrary.Delay` 2.0)
  (`self.K2_DestroyActor`))

(event `Stop Smoke Movement`
  (goto _label))

(fn `UserConstructionScript`)